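; BP_EVIL_ANYA is an AI enemy that chases BP_TopdownChar on sight and otherwise wanders.
; PawnSensing starts the chase and plays audio once per pursuit, while a retriggerable delay clears the sighting flag when detections stop.
; Tick uses delays to confirm lost sight, fade the audio and re-arm it, and to send idle moves to random reachable points nearby.
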(event OnSeePawn(PawnSensing)
  (params (Pawn :type Pawn%20Object%20Reference))
  (bind _asbp_topdown_char (Utilities|Casting|CastToBP_TopdownChar Pawn))
  (Utilities|FlowControl|Sequence
    (:then_0
      (Variables|Default|SetSeeEnemy? true)
      (Variables|Default|SetIsChasing? true)
      (AI|AIMoveTo self "0, 0, 0" _asbp_topdown_char 5.0 false
        (:then
          (Utilities|FlowControl|DoOnce false
            (:Completed
              (Audio|Components|Audio|Play (Variables|Default|GetAudio) 0.0))))))
    (:then_1
      (Utilities|FlowControl|RetriggerableDelay 0.6)
      (Variables|Default|SetSeeEnemy? false))))

(event EventBeginPlay
  ;[1 1 1] Create Audio Ref
  (bind _returnvalue (AddComponent|AddAudioComponent false))
  (Audio|Components|Audio|Stop _returnvalue)
  (Variables|Default|SetAudio _returnvalue))

(event EventTick
  (params (DeltaSeconds :type Float%20%28single-precision%29))
  (Utilities|FlowControl|Sequence
    (:then_0
      (if (not (Variables|Default|GetSeeEnemy?))
        (Utilities|FlowControl|Delay 0.4)
        (if (not (Variables|Default|GetSeeEnemy?))
          (Audio|Components|Audio|FadeOut (Variables|Default|GetAudio) 5.0 0.0 "Linear" :!class /Script/Engine.AudioComponent)
          (Variables|Default|SetIsChasing? false)
          (Utilities|FlowControl|DoOnce false) ; enters at Reset
        )))
    (:then_1
      (if (not (Variables|Default|GetIsChasing?))
        (Utilities|FlowControl|Delay (Math|Random|RandomFloatinRange 2.0 5.0))
        (AI|AIMoveTo self (.RandomLocation (AI|Navigation|GetRandomReachablePointinRadius (Transformation|GetActorLocation) 1.5e+03 0 0)) 0 5.0 false)))))

(event Collision|EventActorBeginOverlap
  (params (OtherActor :type Actor%20Object%20Reference)))

(fn ConstructionScript)