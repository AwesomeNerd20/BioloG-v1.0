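; GM_MAZE is the maze level's game mode Blueprint, handling the key tally and a start countdown.
; On BeginPlay it records the number of Collectible_KeyBP actors as total and remaining keys, shows a countdown widget and disables player input.
; A looping one-second timer decrements the count, updates the text and plays a shutter sound.
; At zero it clears the timer, removes the widget and restores input.
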(event Custom|Take%20Countdown
  (Math|Integer|DecrementInt (Variables|Default|Getcount)
    (:%20%20
      (Rendering|Components|TextRender|SetText (Variables|/Game/StarterContent/BioloG/Blueprints/WBP_CountdownTimer.WBP_CountdownTimer_C|Gettxt_countdown (Variables|Default|Getcountdown%20widget)) (Utilities|Text|ToText(Integer) (Variables|Default|Getcount)))
      (Audio|PlaySound2D "/Engine/VREditor/Sounds/UI/Camera_Shutter.Camera_Shutter" 1.0 1.0 0.0 0 0)
      (if (<= (Variables|Default|Getcount) 0)
        (Utilities|Time|ClearandInvalidateTimerbyHandle (stale EventBeginPlay _returnvalue_2))
        (Widget|RemovefromParent (Variables|Default|Getcountdown%20widget))
        (Input|EnableInput (Game|GetPlayerCharacter 0) (Game|GetPlayerController 0))))))

(event EventBeginPlay
  (Utilities|FlowControl|Sequence
    (:then_0
      (bind _outactors (Actor|GetAllActorsOfClass "/Game/Dhitter_Files/Maze_Elements/Keyllectible/Collectible_KeyBP.Collectible_KeyBP_C"))
      (bind _output_get (Variables|Default|SetKeys%20Left (Utilities|Array|Length _outactors)))
      (Variables|Default|SetTotal%20Keys _output_get))
    (:then_1
      (bind _returnvalue (UserInterface|CreateWidget "/Game/StarterContent/BioloG/Blueprints/WBP_CountdownTimer.WBP_CountdownTimer_C"))
      (bind _output_get_2 (Variables|Default|Setcountdown%20widget _returnvalue))
      (UserInterface|Viewport|AddtoViewport _output_get_2 0)
      (bind _returnvalue_2 (Utilities|Time|SetTimerbyEvent (delegate Custom|Take%20Countdown) 1.0 true))
      (Input|DisableInput (Game|GetPlayerCharacter 0) (Game|GetPlayerController 0)))))

(fn ConstructionScript)